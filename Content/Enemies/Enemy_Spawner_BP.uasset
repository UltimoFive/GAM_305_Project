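; Destructible enemy spawner that spawns Repoduction_Enemy_BP actors beside itself after a per-instance startup delay.
; A timed Delay loop keeps spawning while its enemy count is below a fixed cap, passing each enemy a reference back to the spawner.
; Damage drains its Health; at zero it sets IsDestroyed on the first enemy of that class found in the world, then destroys itself.
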(event `self.ReceiveBeginPlay`
  ; Spawner Enemy Delay before Spawning Enemies, Unique per Spawner
  (`KismetSystemLibrary.Delay` (`self.Delay_Duration`))
  (`self.SpawnEnemy`))

(event `SpawnEnemy`
  (bind (_returnvalue_location _returnvalue_rotation) (`KismetMathLibrary.BreakTransform` (`self.GetTransform`)))
  ; Spawn Enemy from Spawner
  (if (< (`self.Number of enemies`) 4) :!label _label
    (bind _returnvalue (`|SpawnActorFromClass` "/Game/Enemies/Repoduction_Enemy_BP.Repoduction_Enemy_BP_C" (`KismetMathLibrary.MakeTransform` (+ _returnvalue_location (30.0 0.0 0.0)) _returnvalue_rotation) "AdjustIfPossibleButAlwaysSpawn" "MultiplyWithRoot" null null))
    (set `/Game/Enemies/Repoduction_Enemy_BP.Spawner` self _returnvalue)
    (set `self.Number of enemies` (+ (`self.Number of enemies`) 1))
    (`KismetSystemLibrary.Delay` 3.0)
    (goto _label)
    (else
      (`KismetSystemLibrary.Delay` 3.0)
      (goto _label))))

(event `self.ReceiveAnyDamage`
  (params (Damage :type "Float (single-precision)") (DamageType :type "DamageType Object Reference") (InstigatedBy :type "Controller Object Reference") (DamageCauser :type "Actor Object Reference"))
  ; Damage Taken Mechanic
  (set `self.Health` (- (`self.Health`) Damage))
  (if (<= (`self.Health`) 0.0)
    (bind _outactors (`GameplayStatics.GetAllActorsOfClass` "/Game/Enemies/Repoduction_Enemy_BP.Repoduction_Enemy_BP_C"))
    (set `/Game/Enemies/Repoduction_Enemy_BP.isDestroyed?` true (`|GetArrayItem` _outactors))
    (`self.K2_DestroyActor`)))

(fn `UserConstructionScript`)