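; Ranged enemy actor for the virus hunting game mode that fires projectiles and can be killed by damage.
; It increments the Virus_Hunting_Sim AmountLeft counter on BeginPlay and decrements it when its Health runs out, then destroys itself.
; StartShooting and StopShooting events toggle a looping FireRate timer on AIShoot, which plays a pistol sound and spawns Enemy_Projectile_BP from its arrow component.
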(event `self.ReceiveBeginPlay`
  (bind _asvirus_hunting_sim (cast `/Game/Maps/Virus_Hunting_Sim` (`GameplayStatics.GetGameMode`)))
  (set `/Game/Maps/Virus_Hunting_Sim.Amount_Left` (+ (`/Game/Maps/Virus_Hunting_Sim.Amount_Left` _asvirus_hunting_sim) 1) _asvirus_hunting_sim))

(event `self.ReceiveAnyDamage`
  (params (Damage :type "Float (single-precision)") (DamageType :type "DamageType Object Reference") (InstigatedBy :type "Controller Object Reference") (DamageCauser :type "Actor Object Reference"))
  ; Damage Taken Mechanic
  (set `self.Health` (- (`self.Health`) Damage))
  (if (<= (`self.Health`) 0.0)
    (bind _asvirus_hunting_sim (cast `/Game/Maps/Virus_Hunting_Sim` (`GameplayStatics.GetGameMode`)))
    (set `/Game/Maps/Virus_Hunting_Sim.Amount_Left` (- (`/Game/Maps/Virus_Hunting_Sim.Amount_Left` _asvirus_hunting_sim) 1) _asvirus_hunting_sim)
    (`self.K2_DestroyActor`)))

(event `StopShooting`
  (`KismetSystemLibrary.K2_ClearTimer` null "AIShoot"))

(event `StartShooting`
  (`KismetSystemLibrary.K2_SetTimer` null "AIShoot" (`self.Fire_Rate`) true))

(event `AIShoot`
  (`GameplayStatics.PlaySoundAtLocation` "/Game/Player/Pistol_Shot_WAV.Pistol_Shot_WAV" (`self.K2_GetActorLocation`) (struct) 0.2 1.0 0.0 null null null null)
  (`|SpawnActorFromClass` "/Game/Enemies/Ranged_Enemy/Enemy_Projectile_BP.Enemy_Projectile_BP_C" (`SceneComponent.K2_GetComponentToWorld` (`self.Arrow1`)) "Undefined" "MultiplyWithRoot" self null))

(fn `UserConstructionScript`)