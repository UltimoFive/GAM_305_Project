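; Reproduction enemy Blueprint that wanders between tagged actors and can be killed by damage.
; On BeginPlay it sets starting health, moves via AIMoveTo to a random actor with its tag, then pauses and repeats after each successful move.
; AnyDamage subtracts health and destroys the actor at zero or below.
; The Spawner's enemy-count decrement sits in an else branch that rechecks for zero health, so it never runs.
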(event `self.ReceiveBeginPlay`
  ; Movement OverRide
  (set `self.Health` 50.0)
  (bind _outactors (`GameplayStatics.GetAllActorsWithTag` (`self.Tag`) :!label _label))
  (`|AIMoveTo` self (0.0 0.0 0.0) (`KismetArrayLibrary.Array_Random` _outactors)
    (:`OnSuccess`
      (`KismetSystemLibrary.Delay` 2.0)
      (goto _label))))

(event `self.ReceiveAnyDamage`
  (params (Damage :type "Float (single-precision)") (DamageType :type "DamageType Object Reference") (InstigatedBy :type "Controller Object Reference") (DamageCauser :type "Actor Object Reference"))
  ; Damage Taken Mechanic OverRide
  (set `self.Health` (- (`self.Health`) Damage))
  (if (<= (`self.Health`) 0.0)
    (`self.K2_DestroyActor`)
    (elif (and (<= (`self.Health`) 0.0) (== (`self.isDestroyed?`) true))
      (set `/Game/Enemies/Enemy_Spawner_BP.Number of enemies` (- (`/Game/Enemies/Enemy_Spawner_BP.Number of enemies` (`self.Spawner`)) 1) (`self.Spawner`))
      (`self.K2_DestroyActor`))))

(fn `UserConstructionScript`
  (`parent.UserConstructionScript`))